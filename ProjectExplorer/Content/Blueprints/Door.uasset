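; Interactive door Blueprint that the player opens and closes with the E key while inside its trigger box, unless it is locked.
; Trigger overlap enables or disables input for the first player controller and toggles visibility of two text prompts.
; E flips the Open flag, updates both prompts and plays or reverses the DoorRotation timeline, which drives the door's relative yaw.
; The node setting the prompts to "Locked" is unconnected, so it never runs.
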(event OnComponentBeginOverlap(TriggerBox)
  (params (OtherActor :type Actor%20Object%20Reference) (OtherComp :type Primitive%20Component%20Object%20Reference) (OtherBodyIndex :type Integer) (bFromSweep :type Boolean) (SweepResult :type Hit%20Result%20Structure%20%28by%20ref%29))
  (Input|EnableInput (Game|GetPlayerController 0))
  (Rendering|ToggleVisibility (Variables|Default|GetDoorText_002) false))

(event OnComponentEndOverlap(TriggerBox)
  (params (OtherActor :type Actor%20Object%20Reference) (OtherComp :type Primitive%20Component%20Object%20Reference) (OtherBodyIndex :type Integer))
  (Input|DisableInput (Game|GetPlayerController 0))
  (Rendering|ToggleVisibility (Variables|Default|GetDoorText_002) false))

(event Input|KeyboardEvents|E
  (:Pressed
    (if (not (Variables|Default|GetLocked))
      (if (Variables|Default|GetOpen)
        (Variables|Default|SetOpen false)
        (Rendering|Components|TextRender|SetText (Variables|Default|GetDoorText_002) "Press E to open")
        (bind _doorrot (Timeline|DoorRotation Reverse)
          (:Update
            (Transformation|SetRelativeRotation (Variables|Default|GetDoor) (Class|KismetMathLibrary|MakeRot 0.0 _doorrot 0.0) false)))
        (else
          (Variables|Default|SetOpen true)
          (Rendering|Components|TextRender|SetText (Variables|Default|GetDoorText_001) "Press E to close")
          (Timeline|DoorRotation Play))))))

(fn ConstructionScript)